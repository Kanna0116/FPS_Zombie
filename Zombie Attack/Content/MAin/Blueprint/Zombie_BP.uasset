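; Zombie enemy Blueprint that chases the player, attacks and dies.
; From BeginPlay it loops AI MoveTo on the player controller and an attack montage, retrying failed moves, while pawn sensing sets walk speed.
; Point damage reduces health and plays hit reactions or triggers death, but only runs when IsDead is already true.
; Death stops movement, plays a dying montage and loosens collision; attacks apply no damage here.
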(event OnSeePawn(PawnSensing)
  (params (Pawn :type Pawn%20Object%20Reference))
  ;[1 1 1] Zombie Move Ment
  (Variables|/Script/Engine.CharacterMovementComponent|SetMaxWalkSpeed (Variables|Character|GetCharacterMovement) 3.6e+02))

(event Custom|Death
  ;[1 1 1] Zombie Death
  (Variables|Default|SetIs%20Dead? true)
  (Components|Movement|StopMovementImmediately (Variables|Character|GetCharacterMovement))
  (Animation|Montage|PlayMontage (Variables|Character|GetMesh) "/Game/MAin/Zombie_Animation/zombie_dying_Montage.zombie_dying_Montage"
    (:then
      (Collision|SetCollisionResponsetoChannel (Variables|Collision|GetCapsuleComponent) "ECC_Pawn" "ECR_Overlap")
      (Collision|SetCollisionEnabled (Variables|Character|GetMesh) "NoCollision"))))

(event Custom|AttackPlayer
  ;[1 1 1] AttackPlayer
  ;;[1 1 1] Comment
  (Animation|Montage|PlayMontage (Variables|Character|GetMesh) "/Game/MAin/Zombie_Animation/zombie_attack_Montage.zombie_attack_Montage"
    (:OnCompleted
      (CallFunction|RuntoPlayer))))

(event Custom|RunToPlayer
  ;[1 1 1] Chase Player Logic
  (if (not (Variables|Default|GetIs%20Dead?))
    (AI|AIMoveTo self "0, 0, 0" (Game|GetPlayerController 0) 4e+01 false
      (:OnSuccess
        (CallFunction|AttackPlayer))
      (:OnFail
        (CallFunction|RuntoPlayer)))))

(event EventBeginPlay
  ;[1 1 1] Event Begin
  (CallFunction|RuntoPlayer))

(event Game|Damage|EventPointDamage
  (params (Damage :type Float%20%28single-precision%29) (DamageType :type Damage%20Type%20Object%20Reference) (HitLocation :type Vector :default "0, 0, 0") (HitNormal :type Vector :default "0, 0, 0") (HitComponent :type Primitive%20Component%20Object%20Reference) (BoneName :type Name :default "None") (ShotFromDirection :type Vector :default "0, 0, 0") (InstigatedBy :type Controller%20Object%20Reference) (DamageCauser :type Actor%20Object%20Reference) (HitInfo :type Hit%20Result%20Structure%20%28by%20ref%29))
  ;[1 1 1] Apply damage To Zomvie
  (if (Variables|Default|GetIs%20Dead?)
    (if (<= (Variables|Default|GetHealth) 0.0)
      (CallFunction|Death)
      (else
        (bind _output_get (Variables|Default|SetHealth (- (Variables|Default|GetHealth) Damage)))
        (Development|PrintString (Utilities|String|ToString(Float) _output_get))
        (if (<= _output_get 0.0)
          (CallFunction|Death)
          (else
            (Animation|Montage|PlayMontage (Variables|Character|GetMesh) "/Game/MAin/Zombie_Animation/Zombie_Reaction_Hit_mixamo_com_Montage.Zombie_Reaction_Hit_mixamo_com_Montage")))))))

(event EventTick
  (params (DeltaSeconds :type Float%20%28single-precision%29)))

(event Collision|EventActorBeginOverlap
  (params (OtherActor :type Actor%20Object%20Reference)))

(fn ConstructionScript)